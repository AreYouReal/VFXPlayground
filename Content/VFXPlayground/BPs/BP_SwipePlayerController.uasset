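; BP_SwipePlayerController is a player controller that turns touch swipes into rock-paper-scissors turns.
; It caches BP_GameMode on BeginPlay and forwards touch press, move and release, with position and finger index, to its SwipeComponent.
; On release it passes the component's RPSTURN value to the game mode's Turn function and prints the returned result.
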(event `self.ReceiveTick`
  (params (DeltaSeconds :type "Float (single-precision)")))

(event `self.ReceiveBeginPlay`
  (bind _asbp_game_mode (cast `/Game/VFXPlayground/BPs/BP_GameMode` (`GameplayStatics.GetGameMode`)))
  (set `self.GM` _asbp_game_mode))

(event `InputTouch`
  (params (Location :type "Vector Structure") (FingerIndex :type "ETouchIndex Enum"))
  (bind _swipecomponent (`self.SwipeComponent`))
  (:`Pressed`
    (`/Game/VFXPlayground/BPs/SwipeComponent.OnPointerPress` _swipecomponent Location FingerIndex))
  (:`Released`
    (`/Game/VFXPlayground/BPs/SwipeComponent.OnPointerRelease` _swipecomponent Location FingerIndex)
    (bind _result (`/Game/VFXPlayground/BPs/BP_GameMode.Turn` (`self.GM`) (`/Game/VFXPlayground/BPs/SwipeComponent.RPS_TURN` (`self.SwipeComponent`))))
    (`KismetSystemLibrary.PrintString` (`KismetStringLibrary.Conv_IntToString` _result)))
  (:`Moved`
    (`/Game/VFXPlayground/BPs/SwipeComponent.OnPointerMove` _swipecomponent Location FingerIndex)))

(fn `UserConstructionScript`)
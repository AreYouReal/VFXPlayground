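; Game mode for the VFX Playground that registers player heroes and resolves rock-paper-scissors turns against a random AI pick.
; When a new player starts, it lazily caches the game state, then adds the pawn's VSHero to it.
; Turn maps both choices through nested switches to a win, loss or draw value, although matching middle choices return a win instead of a draw.
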(event `self.ReceiveBeginPlay`)

(event `self.HandleStartingNewPlayer`
  (params (NewPlayer :type "PlayerController Object Reference"))
  (`self.CatchGameStateRef`)
  (`parent.HandleStartingNewPlayer` NewPlayer)
  (bind _asmy_player_pawn (cast `/Game/VFXPlayground/BPs/My_PlayerPawn` (`Controller.K2_GetPawn` NewPlayer)))
  (`/Game/VFXPlayground/BPs/MyGameState.AddHero` (`self.MyGameState`) (`/Game/VFXPlayground/BPs/My_PlayerPawn.VSHero` _asmy_player_pawn)))

(fn `CatchGameStateRef`
  (`/Engine/EditorBlueprintResources/StandardMacros.IsValid` (`self.MyGameState`)
    (:`Is Valid`
      (`KismetSystemLibrary.PrintString` "Game state ref is valid"))
    (:`Is Not Valid`
      (`KismetSystemLibrary.PrintString` "Game State Ref is not valid!" true true (struct :`R` 1.0 :`G` 0.050066 :`A` 1.0))
      (bind _asmy_game_state (cast `/Game/VFXPlayground/BPs/MyGameState` (`GameplayStatics.GetGameState`))
        (:`then`
          (set `self.MyGameState` _asmy_game_state)
          (`KismetSystemLibrary.PrintString` "Set Game State Ref"))
        (:`CastFailed`
          (`KismetSystemLibrary.PrintString` "Unable to cast game state" true true (struct :`R` 1.0 :`G` 0.039736 :`A` 1.0)))))))

(fn `Turn`
  (params (RPSTurn :type Integer))
  (returns (Result :type Integer))
  (locals (ReturnValue :type Integer) (UserChoise :type Integer) (AIChoise :type Integer))
  (bind _aichoise (`local.AIChoise`))
  (bind _output_get (set `local.UserChoise` RPSTurn))
  (bind _output_get_2 (set `local.AIChoise` (`KismetMathLibrary.RandomInteger` 3)))
  (`KismetSystemLibrary.PrintString` (`KismetStringLibrary.Concat_StrStr` (`KismetStringLibrary.Conv_IntToString` _output_get) " vs " (`KismetStringLibrary.Conv_IntToString` _output_get_2)))
  (switch `int` (`local.UserChoise`)
    (:`0`
      (switch `int` _aichoise
        (:`0`
          (set `local.ReturnValue` 0))
        (:`1`
          (set `local.ReturnValue` -1))
        (:`2`
          (set `local.ReturnValue` 1))))
    (:`1`
      (switch `int` _aichoise
        (:`0`
          (set `local.ReturnValue` 1))
        (:`1`
          (set `local.ReturnValue` 1))
        (:`2`
          (set `local.ReturnValue` -1))))
    (:`2`
      (switch `int` _aichoise
        (:`0`
          (set `local.ReturnValue` -1))
        (:`1`
          (set `local.ReturnValue` 1))
        (:`2`
          (set `local.ReturnValue` 0)))))
  (return (`local.ReturnValue`)))

(fn `UserConstructionScript`)